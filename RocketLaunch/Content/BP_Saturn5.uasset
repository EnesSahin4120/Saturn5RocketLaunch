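; BP_Saturn5 is a Saturn V rocket Blueprint that starts a simulated launch shortly after play begins.
; The construction script wires its Atmosphere and Rocket references into RocketSimulator, then hands that simulator to RocketHUD.
; On BeginPlay, a short delay precedes calls to Launch and SetSimulate on RocketSimulator.
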(event EventBeginPlay
  (bind _rocketsimulator (Variables|Default|GetRocketSimulator))
  (Utilities|FlowControl|Delay 2.0)
  (Class|RocketSimulator|Launch _rocketsimulator)
  (Class|RocketSimulator|SetSimulate _rocketsimulator))

(fn ConstructionScript
  (Variables|/Script/RocketLaunch.RocketSimulator|SetAtmosphere (Variables|Default|GetRocketSimulator) (Variables|Default|GetAtmosphere))
  (Variables|/Script/RocketLaunch.RocketSimulator|SetRocket (Variables|Default|GetRocketSimulator) (Variables|Default|GetRocket))
  (Variables|/Script/RocketLaunch.RocketHUD|SetRocketSimulator (Variables|Default|GetRocketHUD) (Variables|Default|GetRocketSimulator)))